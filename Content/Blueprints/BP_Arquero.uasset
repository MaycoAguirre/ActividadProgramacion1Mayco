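; BP_Arquero is an archer actor that spawns arrows (flechas) and marks its position with a long-lasting debug box on BeginPlay.
; SpawnFlecha spawns an actor at the archer's location with a supplied rotation, passing it the stored VelocidadFlecha.
; FlechaVelocidad builds that velocity vector by scaling Velocidad by a speed parameter.
; Neither function is called within this Blueprint, and its Tick and overlap events are empty.
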(event EventBeginPlay
  (Rendering|Debug|DrawDebugBox :Center (Transformation|GetActorLocation) :Extent "30.000000,30.000000,30.000000" :Duration 3.6e+03 :Thickness 1e+01))

(event Collision|EventActorBeginOverlap
  (params (OtherActor :type Actor%20Object%20Reference)))

(event EventTick
  (params (DeltaSeconds :type Float%20%28single-precision%29)))

(fn ConstructionScript)

(fn SpawnFlecha
  (params (NewParam :type Rotator))
  (Game|SpawnActorfromClass "/Game/Blueprints/BP_Flecha.BP_Flecha_C" (Math|Transform|MakeTransform (Transformation|GetActorLocation) NewParam "1.000000,1.000000,1.000000") "Undefined" "MultiplyWithRoot" 0 (Variables|Default|GetVelocidadFlecha) 0))

(fn FlechaVelocidad
  (params (velocidadFlecha :type Float%20%28double-precision%29) (velocidad :type Vector))
  (bind _output_get (Variables|Default|SetFlecha%20velocidad1 velocidadFlecha))
  (Variables|Default|SetVelocidadFlecha (Math|Vector|MakeVector (* (.x velocidad) _output_get) (* (.y velocidad) _output_get) (* (.z velocidad) _output_get))))